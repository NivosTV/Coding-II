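; BP_EnemyBase is a base enemy character providing attack, aggro, damage and patrol behavior.
; Attack plays a hook montage and fires AttackFinished on completion or interruption, while aggro swaps the mesh material and sets a flag.
; Point damage reduces health and, at zero, ragdolls the mesh with a radial impulse.
; Helpers set walk speed, return attack and strafe ranges, and step back and forth along a patrol spline's points.
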(event `Attack`
  (`KismetSystemLibrary.PrintText` "Attacking")
  (`|PlayMontage` (`self.Mesh`) "/Game/CloseCombatAnimSet/Animations/InPlace/Attacks/NinjaLeftHook_Montage.NinjaLeftHook_Montage"
    (:`OnCompleted`
      _)
    (:`OnInterrupted`
      _))
  (`self.AttackFinished`))

(event `self.ReceiveBeginPlay`
  (set `self.Original Material` (`PrimitiveComponent.GetMaterial` (`self.Mesh`) 0)) ; save the original material
)

(event `GetAggro`
  ; Aggro
  (`PrimitiveComponent.SetMaterial` (`self.Mesh`) 0 "/AnimationSharing/AnimSharingRed.AnimSharingRed")
  (set `self.Aggroed` true))

(event `LoseAggro`
  ; Aggro
  (`PrimitiveComponent.SetMaterial` (`self.Mesh`) 0 (`self.Original Material`))
  (set `self.Aggroed` false))

(event `Set Walk Speed`
  (params (Speed :type "Float (double-precision)" :default 400.0))
  (set `CharacterMovementComponent.MaxWalkSpeed` Speed (`self.CharacterMovement`)))

(event `self.ReceivePointDamage`
  (params (Damage :type "Float (single-precision)") (DamageType :type "DamageType Object Reference") (HitLocation :type "Vector Structure") (HitNormal :type "Vector Structure") (HitComponent :type "PrimitiveComponent Object Reference") (BoneName :type Name) (ShotFromDirection :type "Vector Structure") (InstigatedBy :type "Controller Object Reference") (DamageCauser :type "Actor Object Reference") (HitInfo :type "HitResult Structure (by ref)"))
  (`KismetSystemLibrary.PrintText` (`|FormatText` "{Instagator} hit me for {DMG} damage!" InstigatedBy Damage))
  (bind _output_get (set `self.Health` (- (`self.Health`) Damage)))
  (if (<= _output_get 0.0)
    (`KismetSystemLibrary.PrintText` "I am dead." true true (struct :`R` 1.0 :`G` 0.000151 :`B` 0.039595 :`A` 1.0))
    (`self.Ragdoll` ShotFromDirection)))

(event `Ragdoll`
  (params (Origin :type "Vector Structure"))
  (bind _mesh (`self.Mesh`))
  (`PrimitiveComponent.SetSimulatePhysics` _mesh true)
  (`PrimitiveComponent.AddRadialImpulse` _mesh (+ Origin (0.0 0.0 -50.0)) 500.0 50000.0 "RIF_Constant" false)
  (`CharacterMovementComponent.DisableMovement` (`self.CharacterMovement`)))

(fn `GetIdealRange`
  (returns (AttackRange :type "Float (double-precision)") (StrafeRange :type "Float (double-precision)"))
  (return (`self.Attack Range`) (`self.Strafe Range`)))

(fn `GetPatrolPointLocation`
  (returns (Location :type "Vector Structure"))
  (set `self.Patrol Index` (+ (`self.Patrol Index`) (`self.Direction`)))
  (if (>= (`self.Patrol Index`) (- (`SplineComponent.GetNumberOfSplinePoints` (`/Game/AI_Blueprints/BP_PatrolRoute.Spline` (`self.PatrolRoute`))) 1))
    (set `self.Direction` -1)
    (elif (<= (`self.Patrol Index`) 0)
      (set `self.Direction` 1)))
  (return (`SplineComponent.GetLocationAtSplinePoint` (`/Game/AI_Blueprints/BP_PatrolRoute.Spline` (`self.PatrolRoute`)) (`self.Patrol Index`) "World")))

(fn `UserConstructionScript`)