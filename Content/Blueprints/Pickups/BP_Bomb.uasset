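; BP_Bomb is a pickup item that can be carried, dropped, armed and disarmed.
; Pickup attaches it to the given skeletal mesh's BPI_ItemSocket and disables its collision, while Drop detaches it without restoring collision.
; Primary and secondary use only swap the cylinder's material between red and base to show armed state, with debug text and no explosion logic.
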(event `/Game/Blueprints/BPI_Item.Drop`
  (`self.K2_DetachFromActor` "KeepRelative"))

(event `/Game/Blueprints/BPI_Item.Pickup`
  (params (`Skeletal Mesh` :type "SkeletalMeshComponent Object Reference"))
  (`KismetSystemLibrary.PrintText` "Bomb picked up")
  (`self.K2_AttachToComponent` `Skeletal Mesh` "BPI_ItemSocket" "SnapToTarget" "SnapToTarget" "KeepRelative")
  (`PrimitiveComponent.SetCollisionEnabled` (`self.Collision`) "NoCollision"))

(event `/Game/Blueprints/BPI_Item.UsePrimary`
  (`KismetSystemLibrary.PrintText` "Bomb armed")
  (`PrimitiveComponent.SetMaterial` (`self.Cylinder`) 0 "/Game/Materials/MI_FlatRed.MI_FlatRed"))

(event `/Game/Blueprints/BPI_Item.UseSecondary`
  (`KismetSystemLibrary.PrintText` "Disarmed")
  (`PrimitiveComponent.SetMaterial` (`self.Cylinder`) 0 "/Game/Materials/M_Base.M_Base"))

(fn `UserConstructionScript`)