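; BP_Radio is a radio item that can be picked up, dropped and used to play music.
; Pickup attaches it to the given skeletal mesh's item socket and disables box collision, while Drop detaches it without re-enabling that collision.
; Primary use alternates stopping and playing the audio component via a FlipFlop, and secondary use alternates its sound between two lofi tracks.
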(event `/Game/Blueprints/BPI_Item.Drop`
  (`KismetSystemLibrary.PrintText` "Radio dropped")
  (`self.K2_DetachFromActor` "KeepRelative"))

(event `/Game/Blueprints/BPI_Item.Pickup`
  (params (`Skeletal Mesh` :type "SkeletalMeshComponent Object Reference"))
  (`KismetSystemLibrary.PrintText` "Radio picked up")
  (`self.K2_AttachToComponent` `Skeletal Mesh` "BPI_ItemSocket" "SnapToTarget" "KeepRelative" "KeepRelative")
  (`PrimitiveComponent.SetCollisionEnabled` (`self.Box`) "NoCollision"))

(event `/Game/Blueprints/BPI_Item.UsePrimary`
  (`KismetSystemLibrary.PrintText` "Toggle Radio")
  (`/Engine/EditorBlueprintResources/StandardMacros.FlipFlop`
    (:`A`
      (`AudioComponent.Stop` (`self.Audio`)))
    (:`B`
      (`AudioComponent.Play` (`self.Audio`) 0.0))))

(event `/Game/Blueprints/BPI_Item.UseSecondary`
  (`KismetSystemLibrary.PrintString` "Switch Songs")
  (`/Engine/EditorBlueprintResources/StandardMacros.FlipFlop`
    (:`A`
      (`AudioComponent.SetSound` (`self.Audio`) "/Game/Audio/Lofi_2.Lofi_2"))
    (:`B`
      (`AudioComponent.SetSound` (`self.Audio`) "/Game/Audio/Lofi_1.Lofi_1"))))

(fn `UserConstructionScript`)