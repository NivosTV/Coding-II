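; BP_FlashlightOLD is a flashlight pickup that can be carried, dropped and used.
; Pickup attaches it to the given skeletal mesh's ik_hand_r socket and disables box collision; Drop detaches it in world space without restoring collision.
; Primary use flip-flops the spotlight's intensity between off and on.
; Secondary use flip-flops its color between white and green, labeled night vision, with debug prints on every event.
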(event `/Game/Blueprints/BPI_Item.Drop`
  (`KismetSystemLibrary.PrintText` "Flashlight dropped")
  (`self.K2_DetachFromActor` "KeepWorld" "KeepWorld" "KeepWorld"))

(event `/Game/Blueprints/BPI_Item.Pickup`
  (params (`Skeletal Mesh` :type "SkeletalMeshComponent Object Reference"))
  (`KismetSystemLibrary.PrintText` "Flashlight picked up")
  (`self.K2_AttachToComponent` `Skeletal Mesh` "ik_hand_r" "SnapToTarget" "SnapToTarget" "KeepRelative")
  (`PrimitiveComponent.SetCollisionEnabled` (`self.Box Collision`) "NoCollision"))

(event `/Game/Blueprints/BPI_Item.UsePrimary`
  (bind _spotlight (`self.SpotLight`))
  (`KismetSystemLibrary.PrintText` "Toggle Flashlight Brightness")
  (`/Engine/EditorBlueprintResources/StandardMacros.FlipFlop`
    (:`A`
      (`LightComponent.SetIntensity` _spotlight 0.0))
    (:`B`
      (`LightComponent.SetIntensity` _spotlight 400.0))))

(event `/Game/Blueprints/BPI_Item.UseSecondary`
  (bind _spotlight (`self.SpotLight`))
  (`KismetSystemLibrary.PrintString` "Night Vision")
  (`/Engine/EditorBlueprintResources/StandardMacros.FlipFlop`
    (:`A`
      (`LightComponent.SetLightColor` _spotlight (struct :`R` 1.0 :`G` 1.0 :`B` 1.0 :`A` 1.0) true))
    (:`B`
      (`LightComponent.SetLightColor` _spotlight (struct :`R` 0.06717 :`G` 1.0 :`A` 1.0) true))))

(fn `UserConstructionScript`)