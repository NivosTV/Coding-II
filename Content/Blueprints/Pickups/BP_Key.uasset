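; BP_Key is a key pickup that adds to the player's key count and records its collection for level saving.
; Overlapping SM_Key with BP_ThirdPersonCharacter increments TotalKeys, destroys the key and prints debug messages.
; It then adds itself to AlteredActors in GM_SaveLoad's SGLevelState, after the first of two DestroyActor calls.
; LoadState calls CollectKey, which destroys the actor without changing the count.
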(event `self.SM_Key.OnComponentBeginOverlap`
  (params (OverlappedComponent :type "PrimitiveComponent Object Reference") (OtherActor :type "Actor Object Reference") (OtherComp :type "PrimitiveComponent Object Reference") (OtherBodyIndex :type Integer) (bFromSweep :type Boolean) (SweepResult :type "HitResult Structure (by ref)"))
  (`KismetSystemLibrary.PrintString` "Key - Overlapped")
  (bind _asbp_third_person_character (cast `/Game/ThirdPerson/Blueprints/BP_ThirdPersonCharacter` OtherActor))
  (bind _result (`/Engine/EditorBlueprintResources/StandardMacros.IncrementInt` (`/Game/ThirdPerson/Blueprints/BP_ThirdPersonCharacter.TotalKeys` _asbp_third_person_character))
    (:`  `
      (`self.K2_DestroyActor`)
      (`KismetSystemLibrary.PrintString` (`KismetStringLibrary.Concat_StrStr` "Player has " (`KismetStringLibrary.Conv_IntToString` _result) " keys"))
      (bind _asgm_save_load (cast `/Game/Blueprints/SavingLoading/GM_SaveLoad` (`GameplayStatics.GetGameMode`)))
      (`KismetArrayLibrary.Array_AddUnique` (`/Game/Blueprints/SavingLoading/SG_LevelState.AlteredActors` (`/Game/Blueprints/SavingLoading/GM_SaveLoad.SG_LevelState` _asgm_save_load)) self)
      (`self.K2_DestroyActor`))))

(event `CollectKey`
  (`self.K2_DestroyActor` self))

(event `/Game/Blueprints/BPI_LeverActorSaveable.LoadState`
  (`self.CollectKey`))

(fn `UserConstructionScript`)