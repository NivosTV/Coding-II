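; BP_Door is a locked door that opens when the player's third-person character walks into it carrying at least one key.
; The collision overlap checks the character's key count and, once only, spends a key and plays a timeline.
; The timeline lerps the door mesh's relative Z to lower it out of the way.
; Without keys, it prints a "No Keys" message.
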(event `self.Collision.OnComponentBeginOverlap`
  (params (OverlappedComponent :type "PrimitiveComponent Object Reference") (OtherActor :type "Actor Object Reference") (OtherComp :type "PrimitiveComponent Object Reference") (OtherBodyIndex :type Integer) (bFromSweep :type Boolean) (SweepResult :type "HitResult Structure (by ref)"))
  (bind _asbp_third_person_character (cast `/Game/ThirdPerson/Blueprints/BP_ThirdPersonCharacter` OtherActor))
  (bind _totalkeys (`/Game/ThirdPerson/Blueprints/BP_ThirdPersonCharacter.TotalKeys` _asbp_third_person_character))
  (if (> _totalkeys 0)
    (`/Engine/EditorBlueprintResources/StandardMacros.DoOnce` false
      (:`Completed`
        (`/Engine/EditorBlueprintResources/StandardMacros.DecrementInt` _totalkeys
          (:`  `
            (bind (_direction _door_movement___open) (`Timeline|Door Movement - Open`)
              (:`Update`
                (`SceneComponent.K2_SetRelativeLocation` (`self.Door`) (`KismetMathLibrary.MakeVector` 0.0 0.0 (`KismetMathLibrary.Lerp` 139.0 -200.0 _door_movement___open)) false false)))))))
    (else
      (`KismetSystemLibrary.PrintText` "No Keys" true true (struct :`R` 0.473958 :`G` 0.017176 :`A` 1.0)))))

(fn `UserConstructionScript`)