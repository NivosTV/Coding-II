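; Demo Blueprint of loop and list techniques that prints its progress on screen from BeginPlay.
; A Delay feeding a DoN re-calls DelayLoop up to ten times at one-second intervals, also triggering the While and For loop demos.
; The While loop counts down around a latent Delay, then resets its counter; the For loop indexes a color array to tint messages.
; A ForEach color demo is present but never called.
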(event `self.ReceiveBeginPlay`
  (`KismetSystemLibrary.PrintString` "Loops and List BP Exists")
  (`self.Delay Loop`))

(event `Delay Loop`
  ; Delay Loop
  (`KismetSystemLibrary.PrintText` (`|FormatText` "This has run {count} times" (stale _counter)))
  (`KismetSystemLibrary.Delay` 1.0)
  (bind _counter (`/Engine/EditorBlueprintResources/StandardMacros.Do N` 10)
    (:`Exit`
      (`self.Delay Loop`)
      (`self.StartWhileLoop`)
      (`self.StartForLoop`))))

(event `StartWhileLoop`
  ; While Loop
  (while (> (`self.WhileLoopCounter`) 0)
    (`KismetSystemLibrary.PrintText` (`|FormatText` "There are {count} more uses in this loop" (`self.WhileLoopCounter`)) true true (struct :`R` 1.0 :`G` 0.148759 :`B` 0.092058 :`A` 1.0))
    (`/Engine/EditorBlueprintResources/StandardMacros.DecrementInt` (`self.WhileLoopCounter`)
      (:`  `
        (`KismetSystemLibrary.Delay` 0.2)
        (`KismetSystemLibrary.PrintString` "After delay" true true (struct :`R` 1.0 :`G` 0.926228 :`B` 0.111277 :`A` 1.0)))))
  (set `self.WhileLoopCounter` 10))

(event `StartForEachLoop`
  ; For Each Loop
  (for (_array_element _array_index) (`|MakeArray` (struct :`R` 0.550313 :`B` 1.0 :`A` 1.0) (struct :`R` 1.0 :`B` 0.045733 :`A` 1.0) (struct :`R` 1.0 :`G` 0.947178 :`B` 0.004752 :`A` 1.0) (struct :`G` 1.0 :`B` 0.950559 :`A` 1.0) (struct :`R` 1.0 :`G` 0.372382 :`A` 1.0) (struct :`R` 0.290927 :`G` 1.0 :`B` 0.001552 :`A` 1.0) (struct :`G` 0.032451 :`B` 1.0 :`A` 1.0) :!type "LinearColor Structure")
    (`KismetSystemLibrary.PrintText` (`|FormatText` "This is index #{index}." _array_index) true true _array_element)))

(event `StartForLoop`
  (bind _array (`|MakeArray` (struct :`R` 0.550313 :`B` 1.0 :`A` 1.0) (struct :`R` 1.0 :`B` 0.045733 :`A` 1.0) (struct :`R` 1.0 :`G` 0.947178 :`B` 0.004752 :`A` 1.0) (struct :`G` 1.0 :`B` 0.950559 :`A` 1.0) (struct :`R` 1.0 :`G` 0.372382 :`A` 1.0) (struct :`R` 0.290927 :`G` 1.0 :`B` 0.001552 :`A` 1.0) (struct :`G` 0.032451 :`B` 1.0 :`A` 1.0) :!type "LinearColor Structure"))
  ; For Loop
  (for _index (range (`KismetArrayLibrary.Array_Length` _array))
    (`KismetSystemLibrary.PrintText` (`|FormatText` "This is index #{index}." _index) true true (`|GetArrayItem` _array _index))))

(fn `UserConstructionScript`)