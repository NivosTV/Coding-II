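; Key-locked door Blueprint that opens when the player character walks into its trigger sphere carrying a key.
; On overlap it checks the third-person character's TotalKeys, printing "No keys" when there are none.
; Otherwise a DoOnce spends one key and plays a timeline that lerps the door mesh downward along Z, so it opens once and never closes.
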(event `self.Sphere Collision.OnComponentBeginOverlap`
  (params (OverlappedComponent :type "PrimitiveComponent Object Reference") (OtherActor :type "Actor Object Reference") (OtherComp :type "PrimitiveComponent Object Reference") (OtherBodyIndex :type Integer) (bFromSweep :type Boolean) (SweepResult :type "HitResult Structure (by ref)"))
  ; Door
  (bind _asbp_third_person_character (cast `/Game/ThirdPerson/Blueprints/BP_ThirdPersonCharacter` OtherActor))
  (if (> (`/Game/ThirdPerson/Blueprints/BP_ThirdPersonCharacter.TotalKeys` _asbp_third_person_character) 0)
    (`/Engine/EditorBlueprintResources/StandardMacros.DoOnce` false
      (:`Completed`
        (`/Engine/EditorBlueprintResources/StandardMacros.DecrementInt` (`/Game/ThirdPerson/Blueprints/BP_ThirdPersonCharacter.TotalKeys` _asbp_third_person_character)
          (:`  `
            (bind (_direction _door___movement_open) (`Timeline|Timeline`)
              (:`Update`
                (`SceneComponent.K2_SetRelativeLocation` (`self.Door`) (`KismetMathLibrary.MakeVector` 0.0 0.0 (`KismetMathLibrary.Lerp` 150.0 -140.0 _door___movement_open)) false false)))))))
    (else
      (`KismetSystemLibrary.PrintString` "No keys" true true (struct :`R` 1.0 :`A` 1.0)))))

(fn `UserConstructionScript`)